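; BP_Janissary is a player-folder Blueprint for a Janissary with a simple health and death system.
; BeginPlay sets current health (MevcutCan) from MaxCan.
; HasarAl (take damage) subtracts the given amount and destroys the actor once health reaches zero or below.
; Pressing T calls HasarAl with a fixed amount, apparently as a damage test, while Tick and overlap events are disabled stubs.
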(event `self.ReceiveBeginPlay`
  (set `self.MevcutCan` (`self.MaxCan`)))

(event `Key|T`
  (params (Key :type "Key Structure"))
  (:`Pressed`
    (`self.HasarAl` 50.0)))

(fn `HasarAl`
  (params (Hasarmiktari :type "Float (double-precision)"))
  (bind _output_get (set `self.MevcutCan` (- (`self.MevcutCan`) Hasarmiktari)))
  (if (<= _output_get 0.0)
    (`self.K2_DestroyActor`)))

(fn `UserConstructionScript`
  (`parent.UserConstructionScript`))